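; BP_Kitsune is a player-controlled Blueprint with third-person camera view, movement and look-around through Enhanced Input.
; On BeginPlay it caches its BP_PlayerController, adds the IMC_Player mapping context and sets the view target to the TPSCamera child actor.
; IA_Movement drives movement input along right and forward vectors derived from actor rotation.
; IA_LookAround feeds controller yaw and pitch.
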(event Input|EnhancedActionEvents|EnhancedInputActionIA_Movement
  (params (ActionValue :type Vector%202D%20Structure) (ElapsedSeconds :type Float%20%28double-precision%29) (TriggeredSeconds :type Float%20%28double-precision%29) (InputAction :type Input%20Action%20Object%20Reference :default "/Game/Custom/Player/Input/IA_Movement.IA_Movement"))
  (bind _returnvalue (Transformation|GetActorRotation))
  ;[1 1 1] Movement & LookAround
  (Pawn|Input|AddMovementInput (Math|Vector|GetRightVector (Math|Rotator|MakeRotator (.roll _returnvalue) 0.0 (.yaw _returnvalue))) (.x ActionValue) false)
  (Pawn|Input|AddMovementInput (Math|Vector|GetForwardVector (Math|Rotator|MakeRotator 0.0 0.0 (.yaw (Transformation|GetActorRotation)))) (.y ActionValue) false))

(event Input|EnhancedActionEvents|EnhancedInputActionIA_LookAround
  (params (ActionValue :type Vector%202D%20Structure) (ElapsedSeconds :type Float%20%28double-precision%29) (TriggeredSeconds :type Float%20%28double-precision%29) (InputAction :type Input%20Action%20Object%20Reference :default "/Game/Custom/Player/Input/IA_LookAround.IA_LookAround"))
  ;[1 1 1] Movement & LookAround
  (Pawn|Input|AddControllerYawInput (.x ActionValue))
  (Pawn|Input|AddControllerPitchInput (.y ActionValue)))

(event EventBeginPlay
  ;[1 1 1] Initailize
  (bind _asbp_player_controller (Utilities|Casting|CastToBP_PlayerController (Pawn|GetController)))
  (bind _output_get (Variables|Default|SetPlayer%20Controller _asbp_player_controller))
  (Input|AddMappingContext (PlayerController|LocalPlayerSubsystems|GetEnhancedInputLocalPlayerSubsystem _output_get) "/Game/Custom/Player/Input/IMC_Player.IMC_Player" 0 "(bIgnoreAllPressedKeysUntilRelease=True,bForceImmediately=False,bNotifyUserSettings=False)")
  (Game|Player|SetViewTargetwithBlend (Variables|Default|GetPlayer%20Controller) (Variables|/Script/Engine.ChildActorComponent|GetChildActor (Variables|Default|GetTPSCamera)) 0.0 "VTBlend_Linear" 0.0 false))

(fn ConstructionScript)